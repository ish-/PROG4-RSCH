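; BP_IshDebugPrint is an on-screen debug readout that shows named values through a WB_IshDebugPrint widget created on BeginPlay.
; The ISh-DebugPrint event stores a "Field:Value" string in a map keyed by field, so repeated calls overwrite that entry.
; Tick uses a frame-count modulo based on UpdateEvery to periodically join all entries and pass the text to the widget.
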(event `self.ReceiveBeginPlay`
  (bind _returnvalue (`|CreateWidget` "/Game/Common/Debug/WB_IshDebugPrint.WB_IshDebugPrint_C" (`GameplayStatics.GetPlayerController` 0)))
  (set `self.widget` _returnvalue)
  (`UserWidget.AddToViewport` _returnvalue 0))

(event `ISh- DebugPrint`
  (params (Field :type String) (Value :type String))
  (`BlueprintMapLibrary.Map_Add` (`self.fields`) Field (`KismetStringLibrary.Concat_StrStr` Field ": " Value)))

(event `self.ReceiveTick`
  (params (DeltaSeconds :type "Float (single-precision)"))
  (if (not (`KismetMathLibrary.Conv_IntToBool` (`KismetMathLibrary.Conv_Int64ToInt` (mod (`KismetSystemLibrary.GetFrameCount`) (`KismetMathLibrary.Conv_IntToInt64` (- (`self.UpdateEvery`) 1))))))
    (bind _values (`BlueprintMapLibrary.Map_Values` (`self.fields`)))
    (`/Game/Common/Debug/WB_IshDebugPrint.DebugUpdate` (`self.widget`) (`KismetTextLibrary.Conv_StringToText` (`KismetStringLibrary.JoinStringArray` _values " \n")))))

(fn `UserConstructionScript`)