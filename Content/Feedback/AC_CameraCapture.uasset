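; Camera feedback component that captures the owner's SceneCaptureComponent2D each tick and feeds cached frames to a post-process material.
; Tick lazily creates a ring of viewport-based render targets and dynamic materials, hooking one into the level's PostProcessVolume.
; Frame-count modulo indices send one slot to post-processing and capture into another shifted by CacheOffset, giving a frame delay.
; Each new capture is also drawn through a copy material into an optional CopyToRenderTarget.
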(event `self.ReceiveBeginPlay`)

(event `Init`
  ;[1 1 1] Initialization
  (`self.Set Camera Aspect`)
  (`self.Set Render Targets`)
  (`self.Set Materials`)
  (`self.Set CineCapture`)
  (set `self.Ready` true))

(event `self.ReceiveTick`
  (params (DeltaSeconds :type "Float (single-precision)"))
  (bind (_returnvalue_x _returnvalue_y) (`KismetMathLibrary.BreakVector2D` (`WidgetLayoutLibrary.GetViewportSize`)))
  (bind _returnvalue (`KismetSystemLibrary.GetFrameCount`))
  (bind _copy_midyn (`self.Copy MIDyn`))
  (bind _copy_to_rendertarget (`self.Copy to RenderTarget`))
  (bind _returnvalue_2 (`KismetMathLibrary.Conv_IntToInt64` (`self.Cache Size`)))
  (if (> _returnvalue_y 0.0)
    (if (not (`KismetMathLibrary.Conv_IntToBool` (`KismetArrayLibrary.Array_Length` (`self.RenderTargets`))))
      (`self.Init`))
    (if (`self.Ready`)
      (`self.Send to PP` (`KismetMathLibrary.Conv_Int64ToInt` (mod _returnvalue _returnvalue_2)))
      (bind _output (`self.Capture` (`KismetMathLibrary.Conv_Int64ToInt` (mod (+ _returnvalue (+ (`self.Cache Offset`) 1)) _returnvalue_2))))
      (`/Engine/EditorBlueprintResources/StandardMacros.IsValid` _copy_to_rendertarget
        (:`Is Valid`
          (`MaterialInstanceDynamic.SetTextureParameterValue` _copy_midyn "Tex0" _output)
          (`KismetRenderingLibrary.DrawMaterialToRenderTarget` _copy_to_rendertarget _copy_midyn))))))

(fn `Capture`
  (params (Index :type Integer))
  (returns (Output :type "TextureRenderTarget2D Object Reference"))
  (bind __cinecapture (`self._CineCapture`))
  (bind _output (`|GetArrayItem` (`self.RenderTargets`) Index))
  (set `SceneCaptureComponent2D.TextureTarget` _output __cinecapture)
  (`SceneCaptureComponent2D.CaptureScene` __cinecapture)
  (return _output))

(fn `Send to PP`
  (params (Index :type Integer))
  (returns (Output :type "TextureRenderTarget2D Object Reference"))
  (bind _output (`|GetArrayItem` (`self.RenderTargets`) Index))
  (`MaterialInstanceDynamic.SetTextureParameterValue` (`self.PostProcessing MIDyn`) "CamTex0" _output)
  (return _output))

(fn `Set Camera Aspect`
  (bind (_returnvalue_x _returnvalue_y) (`KismetMathLibrary.BreakVector2D` (`WidgetLayoutLibrary.GetViewportSize`)))
  (bind _returnvalue (`GameUserSettings.GetGameUserSettings`))
  (`/Game/Common/Debug/FL_IshDebugPrint.ISh- Debug Print` "Screen res:" (`KismetStringLibrary.Concat_StrStr` (`KismetStringLibrary.Conv_DoubleToString` _returnvalue_x) " _ " (`KismetStringLibrary.Conv_DoubleToString` _returnvalue_y))))

(fn `Set CineCapture`
  (bind _output_get (set `self._CineCapture` (`Actor.GetComponentByClass` (`self.GetOwner`) "/Script/Engine.SceneCaptureComponent2D")))
  (set `SceneCaptureComponent2D.TextureTarget` (`self.Copy to RenderTarget`) _output_get))

(fn `Set Materials`
  (bind _returnvalue (`KismetMaterialLibrary.CreateDynamicMaterialInstance` (`self.Copy MAT`)))
  (set `self.Copy MIDyn` _returnvalue)
  (bind _returnvalue_2 (`KismetMaterialLibrary.CreateDynamicMaterialInstance` (`self.PostProcessing MAT`)))
  (bind _output_get (set `self.PostProcessing MIDyn` _returnvalue_2))
  (bind _returnvalue_3 (`GameplayStatics.GetActorOfClass` "/Script/Engine.PostProcessVolume"))
  (`/Engine/EditorBlueprintResources/StandardMacros.IsValid` _returnvalue_3
    (:`Is Valid`
      (bind _weightedblendables_array (break `WeightedBlendables` (break `PostProcessSettings` (`PostProcessVolume.Settings` _returnvalue_3))))
      (`KismetArrayLibrary.Array_Set` _weightedblendables_array 0 (make `WeightedBlendable` 1.0 _output_get) true))
    (:`Is Not Valid`
      (`KismetSystemLibrary.PrintString` "NO PostProcessVolume found!" true true (struct :`R` 1.0 :`B` 0.110754 :`A` 1.0)))))

(fn `Set Render Targets`
  (bind (_returnvalue_x _returnvalue_y) (`KismetMathLibrary.BreakVector2D` (`WidgetLayoutLibrary.GetViewportSize`)))
  (bind _highest_dimension (`self.Highest Dimension`))
  (bind _returnvalue (/ _highest_dimension (/ _returnvalue_x _returnvalue_y)))
  (bind (_returnvalue_x_2 _returnvalue_y_2) (`KismetMathLibrary.BreakVector` (`KismetMathLibrary.SelectVector` (`KismetMathLibrary.MakeVector` _returnvalue_x _returnvalue_y) (`KismetMathLibrary.MakeVector` _returnvalue (* _returnvalue _returnvalue_y)) (> _highest_dimension 0))))
  (bind _returnvalue_2 (`GameUserSettings.GetGameUserSettings`))
  (for _index (range (`self.Cache Size`))
    (bind _returnvalue_3 (`KismetRenderingLibrary.CreateRenderTarget2D` (`KismetMathLibrary.FTrunc` _returnvalue_x_2) (`KismetMathLibrary.FTrunc` _returnvalue_y_2)))
    (`KismetArrayLibrary.Array_Set` (`self.RenderTargets`) _index _returnvalue_3 true)))