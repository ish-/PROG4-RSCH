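; Actor that animates a cloud of instanced static meshes drifting and turning on Perlin noise.
; The construction script places InstanceCount instances with random rotations at noise positions scaled by Range, with absolute Z keeping them above the origin.
; Tick rewrites each transform from elapsed time plus a per-index offset, using helper Perlin1to3 to build vectors from three offset 1D samples.
; BeginPlay fills a Rotations array that the graphs never read.
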(event `self.ReceiveBeginPlay`
  (for _index (range (+ (`self.Instance Count`) 1))
    (`KismetArrayLibrary.Array_Set` (`self.rotations`) _index (`self.Perlin1to3` (`KismetMathLibrary.Conv_IntToDouble` _index) 1.0 5432.0) true)))

(event `self.ReceiveTick`
  (params (DeltaSeconds :type "Float (single-precision)"))
  (bind _output_get (set `self.elapsed` (+ DeltaSeconds (`self.elapsed`))))
  (for _index (range (+ (`self.Instance Count`) 1))
    (bind _returnvalue (* _output_get 0.1))
    (bind _returnvalue_2 (`KismetMathLibrary.Conv_IntToDouble` _index))
    (bind (_vec3_x _vec3_y _vec3_z) (`KismetMathLibrary.BreakVector` (`self.Perlin1to3` (+ _returnvalue (* _returnvalue_2 84.806496)) (`self.Range`))))
    (`InstancedStaticMeshComponent.UpdateInstanceTransform` (`self.InstancedStaticMesh`) _index (`KismetMathLibrary.MakeTransform` (`KismetMathLibrary.MakeVector` _vec3_x _vec3_y (`KismetMathLibrary.Abs` _vec3_z)) (`KismetMathLibrary.Conv_VectorToRotator` (+ (`self.Perlin1to3` (+ (* _returnvalue_2 13.0) _returnvalue) 180.0 3624.7391) (`KismetMathLibrary.Conv_RotatorToVector` (.rotation (`InstancedStaticMeshComponent.GetInstanceTransform` (`self.InstancedStaticMesh`) _index false)))))) false false false)))

(fn `Perlin1to3`
  (params (x :type "Float (single-precision)") (amp :type "Float (double-precision)" :default 1.0) (seed :type "Float (double-precision)"))
  (returns (Vec3 :type "Vector Structure"))
  (bind _returnvalue (+ x seed))
  (bind _returnvalue_2 (+ _returnvalue 33.456))
  (return (* (`KismetMathLibrary.MakeVector` (`KismetMathLibrary.PerlinNoise1D` _returnvalue) (`KismetMathLibrary.PerlinNoise1D` _returnvalue_2) (`KismetMathLibrary.PerlinNoise1D` (+ _returnvalue_2 96.1325))) amp)))

(fn `UserConstructionScript`
  (for _index (range (+ (`self.Instance Count`) 1))
    (bind (_vec3_x _vec3_y _vec3_z) (`KismetMathLibrary.BreakVector` (`self.Perlin1to3` (+ 0.0 (* (`KismetMathLibrary.Conv_IntToDouble` _index) 84.806496)))))
    (`InstancedStaticMeshComponent.AddInstance` (`self.InstancedStaticMesh`) (`KismetMathLibrary.MakeTransform` (* (`KismetMathLibrary.MakeVector` _vec3_x _vec3_y (`KismetMathLibrary.Abs` _vec3_z)) (`self.Range`)) (`KismetMathLibrary.RandomRotator` false)) false)))